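; A clickable six-sided die that rolls on BeginPlay and can be selected for scoring combos.
; RollDice, when allowed, picks the result at random first, then passes it and the matching landing rotation to DicePhysicsRoll.
; Clicking toggles the active state, adds or removes the value in GameManagerSubsystem's temporary combo, registers or unregisters the die, and prints score and combo.
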(event Custom|RollDice
  (if (Class|CPPDice|GetCanRollDice)
    (bind _output_get (Variables|Default|SetGeneratedNumber (Math|Random|RandomIntegerinRange 1 6)))
    (Development|PrintString (Utilities|String|ToString(Integer) _output_get))
    (switch int _output_get
      (:1
        (Class|DicePhysicsRollComponent|RolltoRotation (Variables|Default|GetDicePhysicsRoll) _output_get "0, 0, 0"))
      (:2
        (Class|DicePhysicsRollComponent|RolltoRotation (Variables|Default|GetDicePhysicsRoll) _output_get "0.000000,0.000000,90.000000"))
      (:3
        (Class|DicePhysicsRollComponent|RolltoRotation (Variables|Default|GetDicePhysicsRoll) _output_get "-90.000000,0.000000,0.000000"))
      (:4
        (Class|DicePhysicsRollComponent|RolltoRotation (Variables|Default|GetDicePhysicsRoll) _output_get "90.000000,0.000000,0.000000"))
      (:5
        (Class|DicePhysicsRollComponent|RolltoRotation (Variables|Default|GetDicePhysicsRoll) _output_get "0.000000,0.000000,-90.000000"))
      (:6
        (Class|DicePhysicsRollComponent|RolltoRotation (Variables|Default|GetDicePhysicsRoll) _output_get "0.000000,90.000000,180.000000")))))

(event EventBeginPlay
  (CallFunction|RollDice))

(event Collision|EventActorBeginOverlap
  (params (OtherActor :type Actor%20Object%20Reference)))

(event EventTick
  (params (DeltaSeconds :type Float%20%28single-precision%29)))

(event MouseInput|EventActorOnClicked
  (params (ButtonPressed :type Key%20Structure :default "None"))
  (bind _returnvalue (Subsystems|GetGameManagerSubsystem))
  (bind _returnvalue_2 (Subsystems|GetGameManagerSubsystem))
  (if (Class|CPPDice|GetIsActive)
    (Class|CPPDice|SetIsActive false)
    (bind _returnvalue_3 (Class|GameManagerSubsystem|RemoveCombofromTempArray _returnvalue_2 (Variables|Default|GetGeneratedNumber)))
    (bind _returnvalue_4 (Class|GameManagerSubsystem|GetCurrentScore _returnvalue_2 _returnvalue_3))
    (Development|PrintText (Utilities|Text|FormatText "Score: {Score} 
Combo: {Combo}" _returnvalue_4 _returnvalue_3))
    (Class|GameManagerSubsystem|UnregisterDice _returnvalue self)
    (else
      (Class|CPPDice|SetIsActive true)
      (bind _returnvalue_5 (Class|GameManagerSubsystem|AddCombotoTempArray _returnvalue_2 (Variables|Default|GetGeneratedNumber)))
      (bind _returnvalue_6 (Class|GameManagerSubsystem|GetCurrentScore _returnvalue_2 _returnvalue_5))
      (Development|PrintText (Utilities|Text|FormatText "Score: {Score} 
Combo: {Combo}" _returnvalue_6 _returnvalue_5))
      (Class|GameManagerSubsystem|RegisterDice _returnvalue self))))

(fn ConstructionScript)