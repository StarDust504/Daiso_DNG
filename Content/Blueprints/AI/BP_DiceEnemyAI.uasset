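; BP_DiceEnemyAI is the AI opponent that rolls the dice when its turn begins.
; On BeginPlay it finds the BP_TurnManager, binds to its OnTurnChanged event and caches every BP_Dice in the level.
; When the new turn is the AI's, it waits briefly, then activates and rolls each cached die.
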(event Custom|ManageTurnChange
  (params (PreviousTurn :type EDiceTurnOwner%20Enum :default "Player") (NewTurn :type EDiceTurnOwner%20Enum :default "Player") (Reason :type EDiceTurnChangeReason%20Enum :default "GameStarted"))
  (if (Utilities|Enum|Equal(Enum) NewTurn "AI")
    (Utilities|FlowControl|Delay 0.75)
    (for _array_element (Variables|Default|GetDiceArray)
      (Class|CPPDice|SetIsActive _array_element true)
      (Default|RollDice _array_element))))

(event EventBeginPlay
  (bind _returnvalue (Actor|GetActorOfClass "/Game/Blueprints/TurnManager/BP_TurnManager.BP_TurnManager_C"))
  (bind _output_get (Variables|Default|SetTurnManager _returnvalue))
  (EventDispatchers|BindEventtoOnTurnChanged _output_get (EventDispatchers|CreateEvent :!event Custom|ManageTurnChange))
  (bind _outactors (Actor|GetAllActorsOfClass "/Game/Blueprints/Props/Dice/BP_Dice.BP_Dice_C"))
  (Variables|Default|SetDiceArray _outactors))

(event Collision|EventActorBeginOverlap
  (params (OtherActor :type Actor%20Object%20Reference)))

(event EventTick
  (params (DeltaSeconds :type Float%20%28single-precision%29)))

(fn ConstructionScript)