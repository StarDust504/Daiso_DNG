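; BP_Player is the player Blueprint for a turn-based dice game, handling Roll and Pass input.
; On BeginPlay it finds BP_TurnManager and binds to its turn-changed event; its ManageTurnChange event is still empty.
; Roll destroys registered dice through the GameManagerSubsystem and ends the player's turn, with no dice spawning here.
; Pass only prints a debug message.
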(event Custom|ManageTurnChange
  (params (PreviousTurn :type EDiceTurnOwner%20Enum :default "Player") (NewTurn :type EDiceTurnOwner%20Enum :default "Player") (Reason :type EDiceTurnChangeReason%20Enum :default "GameStarted")))

(event Input|EnhancedActionEvents|EnhancedInputActionIA_Pass
  (params (ActionValue :type Boolean) (ElapsedSeconds :type Float%20%28double-precision%29) (TriggeredSeconds :type Float%20%28double-precision%29) (InputAction :type Input%20Action%20Object%20Reference :default "/Game/Player/Input/Actions/IA_Pass.IA_Pass"))
  (:Started
    (Development|PrintString "PASS")))

(event Input|EnhancedActionEvents|EnhancedInputActionIA_Roll
  (params (ActionValue :type Boolean) (ElapsedSeconds :type Float%20%28double-precision%29) (TriggeredSeconds :type Float%20%28double-precision%29) (InputAction :type Input%20Action%20Object%20Reference :default "/Game/Player/Input/Actions/IA_Roll.IA_Roll"))
  (:Started
    (Class|GameManagerSubsystem|DestroyRegisteredDice (Subsystems|GetGameManagerSubsystem))
    (Development|PrintString "ROLL")
    (Class|DiceTurnManager|EndPlayerTurn (Variables|Default|GetTurnManager))))

(event EventBeginPlay
  (bind _returnvalue (Actor|GetActorOfClass "/Game/Blueprints/TurnManager/BP_TurnManager.BP_TurnManager_C"))
  (bind _output_get (Variables|Default|SetTurnManager _returnvalue))
  (EventDispatchers|BindEventtoOnTurnChanged _returnvalue (EventDispatchers|CreateEvent :!event Custom|ManageTurnChange)))

(fn ConstructionScript)